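; BP_GameManager tracks the player's conversation progress and picks the game's ending from accumulated influence.
; UpdateValues adds gained influence, increments the conversation count and, when that count matches the maximum, sorts the total into a good, neutral or bad ending using fixed thresholds.
; Endings are only printed as debug strings, along with the final score.
; A getter and setter store the NPC of the active conversation.
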(fn `GetActiveConversation`
  (returns (NPC :type "/Game/Blueprints/Dialogue/Enums/E_NPCNames Enum"))
  (return (`self.NPC`)))

(fn `SetActiveConversation`
  (params (NPC :type "/Game/Blueprints/Dialogue/Enums/E_NPCNames Enum" :default "NewEnumerator0"))
  (set `self.NPC` NPC))

(fn `UpdateValues`
  (params (InfluenceGained :type Integer))
  (bind _influence (`self.influence`))
  (set `self.influence` (+ InfluenceGained (`self.influence`)))
  (bind _result (`/Engine/EditorBlueprintResources/StandardMacros.IncrementInt` (`self.conversationCount`))
    (:`  `
      (if (== _result (`self.maxConversations`))
        (if (>= _influence 12)
          (`KismetSystemLibrary.PrintString` "Good Ending")
          (elif (>= _influence 6)
            (`KismetSystemLibrary.PrintString` "Neutral Ending")
            (else
              (`KismetSystemLibrary.PrintString` "Bad Ending"))))
        (`KismetSystemLibrary.PrintString` (`KismetStringLibrary.Conv_IntToString` (`self.influence`)))))))

(fn `UserConstructionScript`)